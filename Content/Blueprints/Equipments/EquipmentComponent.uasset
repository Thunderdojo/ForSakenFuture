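; Equipment component that manages a player's equipped item slots and toggles the equipment window widget.
; Items live as ID and quantity in a slot array; AddEquipment writes a slot, first calling RemoveEquipment if its quantity is zero.
; RemoveEquipment spawns the item through the controlled BaseCharacter without clearing the slot.
; AddEquipmentToInventory clears the slot on a successful transfer, or calls RemoveEquipment when the inventory is invalid.
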(fn ToggleEquipment
  (params (PlayerController :type Player%20Controller%20Object%20Reference))
  ;[0.03302 1 0] Open or close the Equipment depending if its allready there or not
  (Variables|Default|SetPlayer%20Controller PlayerController)
  (Utilities|IsValid (Variables|Default|GetEquipmentRef)
    (:Is%20Valid
      (Widget|RemovefromParent (Variables|Default|GetEquipmentRef))
      (Variables|Default|SetEquipmentRef 0))
    (:Is%20Not%20Valid
      (bind _returnvalue (UserInterface|CreateWidget "/Game/UI/Equipments/EquipmentWindow.EquipmentWindow_C" PlayerController))
      (bind _output_get (Variables|Default|SetEquipmentRef _returnvalue))
      (UserInterface|Viewport|AddtoViewport _output_get 0))))

(fn AddEquipment
  (params (ItemID :type Name) (Quantity :type Integer) (SlotNumber :type Integer))
  (bind _equipmentsarray (Variables|Default|GetEquipmentsArray))
  ;[0.08068 1 0] Add Equipment to slot, if there Allready is an item there, spawn it in the world and set the new item
  (if (!= (.quantity (Utilities|Array|Get(acopy) _equipmentsarray SlotNumber)) 0)
    _
    (else
      (CallFunction|RemoveEquipment SlotNumber)))
  (Utilities|Array|SetArrayElem _equipmentsarray SlotNumber (Utilities|Struct|MakeF_SlotStruct ItemID Quantity)))

(fn RemoveEquipment
  (params (SlotNumber :type Integer))
  (bind _equipmentsarray (Variables|Default|GetEquipmentsArray))
  (bind _output (Utilities|Array|Get(acopy) _equipmentsarray SlotNumber))
  (bind (_itemid _quantity) (Utilities|Struct|BreakF_SlotStruct _output))
  ;[1 1 1] Remove the item and spawn it in the world
  (bind _asbase_character (Utilities|Casting|CastToBaseCharacter (Pawn|GetControlledPawn (Variables|Default|GetPlayer%20Controller))))
  (Default|SpawnIteminWorld _asbase_character (Utilities|Struct|MakeF_SlotStruct _itemid _quantity)))

(fn AddEquipmenttoInventory
  (params (Inventory :type Inventory%20Component%20Object%20Reference) (SlotNumber :type Integer))
  (bind _equipmentsarray (Variables|Default|GetEquipmentsArray))
  (bind _output (Utilities|Array|Get(acopy) _equipmentsarray SlotNumber))
  ;[0.2415 1 0.00269] Add Equipment to our inventory if we got one, Else we spawn it to the world
  (Utilities|IsValid Inventory
    (:Is%20Valid
      (bind _success (Default|AddtoInventory Inventory (.itemid _output) (.quantity _output)))
      (if _success
        (Utilities|Array|SetArrayElem :TargetArray _equipmentsarray :Index SlotNumber)))
    (:Is%20Not%20Valid
      (CallFunction|RemoveEquipment SlotNumber))))