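; ProjectileBertha is a projectile that explodes where it stops and deals area damage.
; Its Sphere starts with collision disabled, then switches to query and probe on impact as a large explosion emitter spawns.
; Sphere overlaps call DamageMisile, which applies fixed damage to the sweep result's hit actor rather than the overlap's other actor.
; The actor destroys itself after a short delay, limiting the damage window.
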(event OnProjectileStop(ProjectileMovement)
  (params (ImpactResult :type Hit%20Result%20Structure%20%28by%20ref%29))
  (Collision|SetCollisionEnabled (Variables|Default|GetSphere) "QueryAndProbe")
  (Effects|SpawnEmitteratLocation "/Game/StarterContent/Particles/P_Explosion.P_Explosion" (.Location (Collision|BreakHitResult ImpactResult)) "0.000000,1.000000,0.000000" "10.000000,10.000000,10.000000")
  (Utilities|FlowControl|Delay 0.5)
  (Actor|DestroyActor))

(event OnComponentBeginOverlap(Sphere)
  (params (OverlappedComponent :type Primitive%20Component%20Object%20Reference) (OtherActor :type Actor%20Object%20Reference) (OtherComp :type Primitive%20Component%20Object%20Reference) (OtherBodyIndex :type Integer) (bFromSweep :type Boolean) (SweepResult :type Hit%20Result%20Structure%20%28by%20ref%29))
  (CallFunction|DamageMisile SweepResult))

(event Custom|DamageMisile
  (params (Hit :type Hit%20Result%20Structure%20%28by%20ref%29))
  (Game|Damage|ApplyDamage (.HitActor (Collision|BreakHitResult Hit)) 1e+01 0 0))

(fn ConstructionScript
  (Collision|SetCollisionEnabled (Variables|Default|GetSphere) "NoCollision"))