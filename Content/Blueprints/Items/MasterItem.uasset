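; MasterItem is a pickup item actor, described by an item struct, that characters can find and store in their backpack inventory.
; Overlapping its sensor shows a ScreenMessage prompt naming the item, removed after a delay or when the character leaves.
; Interact adds one item to the backpack's inventory component and destroys the actor on success.
; Without a backpack it switches on item type, with no branches implemented yet.
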(event OnComponentBeginOverlap(Overlapsensor)
  (params (OverlappedComponent :type Primitive%20Component%20Object%20Reference) (OtherActor :type Actor%20Object%20Reference) (OtherComp :type Primitive%20Component%20Object%20Reference) (OtherBodyIndex :type Integer) (bFromSweep :type Boolean) (SweepResult :type Hit%20Result%20Structure%20%28by%20ref%29))
  (Utilities|Casting|CastToBaseCharacter OtherActor)
  (Utilities|IsValid (Variables|Default|GetScreenMessageRef)
    (:Is%20Not%20Valid
      (bind _returnvalue (UserInterface|CreateWidget "/Game/UI/Ingame/ScreenMessage.ScreenMessage_C" 0 (Utilities|Text|ToText(String) (Utilities|String|Append "You found : " (Utilities|String|ToString(Text) (.itemname (Variables|Default|GetItemStruct))) " Press'E' To Interact"))))
      (bind _output_get (Variables|Default|SetScreenMessageRef _returnvalue))
      (UserInterface|Viewport|AddtoViewport _output_get 0)
      (Utilities|FlowControl|Delay 6.0)
      (Utilities|IsValid (Variables|Default|GetScreenMessageRef)
        (:Is%20Valid
          (Widget|RemovefromParent (Variables|Default|GetScreenMessageRef))
          (Variables|Default|SetScreenMessageRef 0))))))

(event OnComponentEndOverlap(Overlapsensor)
  (params (OverlappedComponent :type Primitive%20Component%20Object%20Reference) (OtherActor :type Actor%20Object%20Reference) (OtherComp :type Primitive%20Component%20Object%20Reference) (OtherBodyIndex :type Integer))
  (Utilities|Casting|CastToBaseCharacter OtherActor)
  (Utilities|IsValid (Variables|Default|GetScreenMessageRef)
    (:Is%20Valid
      (Widget|RemovefromParent (Variables|Default|GetScreenMessageRef))
      (Variables|Default|SetScreenMessageRef 0))))

(event EventInteract
  (params (PlayerCharacter :type Base%20Character%20Object%20Reference))
  (bind _backpackref (Variables|/Game/Blueprints/Characters/BaseCharacter.BaseCharacter_C|GetBackPackRef PlayerCharacter))
  ;[1 1 1] TODO: Make it possible to hold things or attach armor or clothes to player even if you do not have a backpack(inventory)
  (Utilities|IsValid _backpackref
    (:Is%20Valid
      (bind (_success _quantity_remaing) (Default|AddtoInventory (Variables|/Game/Blueprints/InvenTory/BackPacks/Master_Backpack.Master_Backpack_C|GetInventoryComponent _backpackref) (Utilities|Struct|MakeSlotStructure (Variables|Default|GetItemStruct) 1)))
      (if _success
        (Actor|DestroyActor)
        (else
          (Variables|Default|SetQuantity%20Remaing _quantity_remaing))))
    (:Is%20Not%20Valid
      (switch Utilities|FlowControl|Switch|SwitchonItemType (.itemtype (Variables|Default|GetItemStruct))))))

(fn ConstructionScript)