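; Bottle is a pickup item that shows an on-screen prompt when a BaseCharacter overlaps its sensor.
; The prompt uses the description from the item's data table row and clears after a delay or when overlap ends.
; Interact adds the item to the player's backpack inventory, destroying the actor on success.
; Without a backpack, it disables collision and attaches the bottle to the character's RightHand socket.
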(event OnComponentBeginOverlap(Overlapsensor)
  (params (OverlappedComponent :type Primitive%20Component%20Object%20Reference) (OtherActor :type Actor%20Object%20Reference) (OtherComp :type Primitive%20Component%20Object%20Reference) (OtherBodyIndex :type Integer) (bFromSweep :type Boolean) (SweepResult :type Hit%20Result%20Structure%20%28by%20ref%29))
  (bind _itemdatacomponent (Variables|Default|GetItemDataComponent))
  (bind _itemid (Variables|/Game/Blueprints/Items/ItemDataComponent.ItemDataComponent_C|GetItemID _itemdatacomponent))
  (Utilities|Casting|CastToBaseCharacter OtherActor)
  (bind _returnvalue (Utilities|GetDataTableRow (.datatable _itemid) (.rowname _itemid))
    (:then
      _)
    (:RowNotFound
      _))
  (Utilities|IsValid (Variables|Default|GetScreenMessageRef)
    (:Is%20Not%20Valid
      (bind _returnvalue_2 (UserInterface|CreateWidget "/Game/UI/Ingame/ScreenMessage.ScreenMessage_C" 0 (Utilities|Text|ToText(String) (Utilities|String|Append "You found : " (Utilities|String|ToString(Text) (.Description (Utilities|Struct|BreakF_ItemStruct _returnvalue))) " Press'E' To Interact"))))
      (bind _output_get (Variables|Default|SetScreenMessageRef _returnvalue_2))
      (UserInterface|Viewport|AddtoViewport _output_get 0)
      (Utilities|FlowControl|Delay 6.0)
      (Utilities|IsValid (Variables|Default|GetScreenMessageRef)
        (:Is%20Valid
          (Widget|RemovefromParent (Variables|Default|GetScreenMessageRef))
          (Variables|Default|SetScreenMessageRef 0))))))

(event OnComponentEndOverlap(Overlapsensor)
  (params (OverlappedComponent :type Primitive%20Component%20Object%20Reference) (OtherActor :type Actor%20Object%20Reference) (OtherComp :type Primitive%20Component%20Object%20Reference) (OtherBodyIndex :type Integer))
  (Utilities|Casting|CastToBaseCharacter OtherActor)
  (Utilities|IsValid (Variables|Default|GetScreenMessageRef)
    (:Is%20Valid
      (Widget|RemovefromParent (Variables|Default|GetScreenMessageRef))
      (Variables|Default|SetScreenMessageRef 0))))

(event EventInteract
  (params (PlayerCharacter :type Base%20Character%20Object%20Reference))
  (bind _self self)
  (bind _itemdatacomponent (Variables|Default|GetItemDataComponent))
  (bind _mesh (Variables|/Script/Engine.Character|GetMesh PlayerCharacter))
  (bind _backpackref (Variables|/Game/Blueprints/Characters/BaseCharacter.BaseCharacter_C|GetBackPackRef PlayerCharacter))
  ;[1 1 1] TODO: Make it possible to hold things or attach armor or clothes to player even if you do not have a backpack(inventory)
  (Utilities|IsValid _backpackref
    (:Is%20Valid
      (bind _success (Default|AddtoInventory (Variables|/Game/Blueprints/InvenTory/BackPacks/Master_Backpack.Master_Backpack_C|GetInventoryComponent _backpackref) (.rowname (Variables|/Game/Blueprints/Items/ItemDataComponent.ItemDataComponent_C|GetItemID _itemdatacomponent)) (Variables|/Game/Blueprints/Items/ItemDataComponent.ItemDataComponent_C|GetQuantity _itemdatacomponent)))
      (if _success
        (Actor|DestroyActor)))
    (:Is%20Not%20Valid
      (Collision|SetActorEnableCollision _self false)
      (Transformation|AttachComponentToComponent _self _mesh "RightHand" "SnapToTarget" "SnapToTarget" "SnapToTarget" true)
      (Transformation|AttachComponentToComponent (Variables|Default|GetItemMesh) _mesh "RightHand" "SnapToTarget" "SnapToTarget" "SnapToTarget" true))))

(fn ConstructionScript)