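; ButterRoute is a route Blueprint that flies a target actor, apparently a butterfly, along a spline in a continuous loop.
; A timeline starts on BeginPlay, lerps distance from zero to the last spline point to set the target's swept world location, and restarts when finished.
; Rotation comes from the local-space tangent at distance zero, so it does not follow the curve.
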(event Custom|Fly%20Butter%20fly
  (bind _spline (Variables|Default|GetSpline))
  (bind _target (Variables|Default|GetTarget))
  (bind _alpha (Timeline|Time PlayFromStart)
    (:Update
      (Transformation|SetActorLocation _target (Spline|GetLocationatDistanceAlongSpline _spline (Math|Float|Lerp 0.0 (Spline|GetDistanceAlongSplineatSplinePoint _spline (- (Spline|GetNumberOfSplinePoints _spline) 1)) _alpha) "World") true false)
      (Transformation|SetActorRotation _target (Math|Conversions|RotationFromXVector (Spline|GetTangentatDistanceAlongSpline _spline 0.0 "Local")) true))
    (:Finished
      (CallFunction|FlyButterFly))))

(event EventBeginPlay
  (CallFunction|FlyButterFly))

(fn ConstructionScript)