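; Inventory component that holds a named array of item slots, adds items to it and toggles its window.
; ToggleInventory opens a backpack or general widget by name, switching input mode and cursor.
; AddToInventory loops per unit through FindSlot, AddToStack or CreateNewStack, re-toggling an open backpack to refresh it.
; The empty-slot check tests only the first slot, AddToStack overwrites rather than increments quantity, and remove and refresh are stubs.
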(event Custom|InitInventory
  (params (Array :type Array%20of%20Slot%20Structure%20Structures) (InventoryName :type String) (ThisInventorySlotCount :type Integer))
  (Variables|Default|SetThisInventorySlots Array)
  (Variables|Default|SetInventoryName InventoryName)
  (Variables|Default|SetThisInventorySlotCount ThisInventorySlotCount))

(fn ToggleInventory
  (params (OwningPlayer :type Player%20Controller%20Object%20Reference))
  (if (Utilities|String|Contains (Variables|Default|GetInventoryName) "backpack")
    (Utilities|IsValid (Variables|Default|GetBPWindowRef)
      (:Is%20Valid
        (Widget|RemovefromParent (Variables|Default|GetBPWindowRef))
        (Variables|Default|SetBPWindowRef 0)
        (Input|SetInputModeGameOnly OwningPlayer false)
        (Variables|/Script/Engine.PlayerController|SetbShowMouseCursor OwningPlayer false))
      (:Is%20Not%20Valid
        (bind _returnvalue (UserInterface|CreateWidget "/Game/UI/Inventory/BackPackWindow.BackPackWindow_C" 0 self))
        (bind _output_get (Variables|Default|SetBPWindowRef _returnvalue))
        (UserInterface|Viewport|AddtoViewport _output_get 0)
        (Input|SetInputModeGameandUI OwningPlayer 0 "DoNotLock" true false)
        (Variables|/Script/Engine.PlayerController|SetbShowMouseCursor OwningPlayer true)))
    (else
      (Utilities|IsValid (Variables|Default|GetInventoryWindowRef)
        (:Is%20Valid
          (Widget|RemovefromParent (Variables|Default|GetInventoryWindowRef))
          (bind _output_get_2 (Variables|Default|SetInventoryWindowRef 0))
          (Input|SetInputModeGameOnly OwningPlayer false)
          (Variables|/Script/Engine.PlayerController|SetbShowMouseCursor OwningPlayer false)
          (return _output_get_2))
        (:Is%20Not%20Valid
          (bind _returnvalue_2 (UserInterface|CreateWidget "/Game/UI/Inventory/InvenToryWindows.InvenToryWindows_C" OwningPlayer self))
          (bind _output_get_3 (Variables|Default|SetInventoryWindowRef _returnvalue_2))
          (UserInterface|Viewport|AddtoViewport _output_get_3 0)
          (Input|SetInputModeGameandUI OwningPlayer 0 "DoNotLock" true false)
          (Variables|/Script/Engine.PlayerController|SetbShowMouseCursor OwningPlayer true)
          (return _output_get_3))))))

(fn RefreshInventoryforUI)

(fn AddtoInventory
  (params (SlotStructure :type Slot%20Structure%20Structure))
  (LocalVariables|SetQuantity_Remaining (.quantity SlotStructure))
  (while (and (> (LocalVariables|GetQuantity_Remaining) 0) (not (LocalVariables|GetLocal_HasFailed)))
    (bind (_index _hasfoundslot) (CallFunction|FindSlot (Utilities|Struct|MakeSlotStructure (.item SlotStructure) (.quantity SlotStructure))))
    (if _hasfoundslot
      (CallFunction|AddtoStack _index (.item SlotStructure) 1)
      (Math|Integer|DecrementInt (LocalVariables|GetQuantity_Remaining))
      (elif (.HasEmptySlot (CallFunction|AnyEmptySlotsAvailable))
        (bind _success (CallFunction|CreateNewStack (Utilities|Struct|MakeSlotStructure (.item SlotStructure) 1)))
        (if _success
          (Math|Integer|DecrementInt (LocalVariables|GetQuantity_Remaining))
          (else
            (LocalVariables|SetLocal_HasFailed true)))
        (else
          (LocalVariables|SetLocal_HasFailed true)))))
  (Utilities|IsValid (Variables|Default|GetBPWindowRef)
    (:Is%20Valid
      (CallFunction|ToggleInventory (Game|GetPlayerController 0))
      (CallFunction|ToggleInventory (Game|GetPlayerController 0)))
    (:Is%20Not%20Valid
      _))
  (return (not (LocalVariables|GetLocal_HasFailed)) (LocalVariables|GetQuantity_Remaining)))

(fn FindSlot
  (params (Slotstructure :type Slot%20Structure%20Structure))
  (for (_array_element _array_index) (Variables|Default|GetThisInventorySlots)
    (if (== (.itemclass (.Item (Utilities|Struct|BreakSlotStructure _array_element))) (.ItemClass (Utilities|Struct|BreakItemStruct (.item Slotstructure))))
      (if (< (.Quantity (Utilities|Struct|BreakSlotStructure _array_element)) (CallFunction|GetMaxStackSize (Utilities|Struct|MakeSlotStructure (.item Slotstructure) 0)))
        (return _array_index true))))
  (return -1 false))

(fn GetMaxStackSize
  (params (Slotstructure :type Slot%20Structure%20Structure))
  (return (Utilities|Struct|BreakItemStruct (.item Slotstructure))))

(fn AddtoStack
  (params (Index :type Integer) (Item%20Item :type Item%20Struct%20Structure) (Item%20Quantity :type Integer))
  (Utilities|Array|SetArrayElem (Variables|Default|GetThisInventorySlots) Index (Utilities|Struct|MakeSlotStructure Item%20Item (+ Item%20Quantity 1))))

(fn AnyEmptySlotsAvailable
  (for (_array_element _array_index) (Variables|Default|GetThisInventorySlots)
    (if (== (.Quantity (Utilities|Struct|BreakSlotStructure _array_element)) 0)
      (return true _array_index)
      (else
        (return false -1)))))

(fn CreateNewStack
  (params (SlotStructure :type Slot%20Structure%20Structure))
  (bind (_hasemptyslot _array_index) (CallFunction|AnyEmptySlotsAvailable))
  (if _hasemptyslot
    (Utilities|Array|SetArrayElem (Variables|Default|GetThisInventorySlots) _array_index (Utilities|Struct|MakeSlotStructure (.item SlotStructure) (.quantity SlotStructure)))
    (return true)
    (else
      (return false))))

(fn RemovefromInvenTory)