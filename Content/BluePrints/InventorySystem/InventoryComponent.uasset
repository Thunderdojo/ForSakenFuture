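; Inventory component that stores item stacks in a slot array and opens or closes their UI window, choosing the backpack widget when its name contains "backpack".
; Adding puts one item on a matching non-full stack or the first empty slot, failing when none is free.
; Removal empties depleted slots, with lookup functions and batch removal for crafting.
; Changes refresh the UI by toggling the window twice, which also switches cursor and input mode.
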(fn ToggleInventory
  (params (Playercontroller :type Player%20Controller%20Object%20Reference))
  ;[0.04647 0.3116 1] Taking care of opening and closing either backpackwindow or inventory window
  ;;[1 0.8897 0] Check if name has backpack in it, if so we open players backpack, else we will open an inventory window for the other
  (if (Utilities|String|Contains (Utilities|String|ToString(Text) (Variables|Default|GetName%20Text)) "backpack")
    (Utilities|IsValid (Variables|Default|GetBackpackwindowRef)
      (:Is%20Valid
        (Widget|RemovefromParent (Variables|Default|GetBackpackwindowRef))
        (Variables|Default|SetBackpackwindowRef 0)
        (Variables|/Script/Engine.PlayerController|SetbShowMouseCursor Playercontroller false)
        (Input|SetInputModeGameOnly Playercontroller false))
      (:Is%20Not%20Valid
        (bind _returnvalue (UserInterface|CreateWidget "/Game/UI/InvenTory/BackpackWindow.BackpackWindow_C" Playercontroller (Variables|Default|GetName%20Text) (Variables|Default|GetIcon) self))
        (bind _output_get (Variables|Default|SetBackpackwindowRef _returnvalue))
        (UserInterface|Viewport|AddtoViewport _output_get 0)
        (Variables|/Script/Engine.PlayerController|SetbShowMouseCursor Playercontroller true)
        (Input|SetInputModeGameandUI Playercontroller 0 "DoNotLock" true false)))
    (else
      (Utilities|IsValid (Variables|Default|GetInventoryWindowRef)
        (:Is%20Valid
          (Widget|RemovefromParent (Variables|Default|GetInventoryWindowRef))
          (Variables|Default|SetInventoryWindowRef 0)
          (Variables|/Script/Engine.PlayerController|SetbShowMouseCursor Playercontroller false)
          (Input|SetInputModeGameOnly Playercontroller false))
        (:Is%20Not%20Valid
          (bind _returnvalue_2 (UserInterface|CreateWidget "/Game/UI/InvenTory/InvenToryWindow.InvenToryWindow_C" 0 (Variables|Default|GetName%20Text) (Variables|Default|GetIcon) self))
          (bind _output_get_2 (Variables|Default|SetInventoryWindowRef _returnvalue_2))
          (UserInterface|Viewport|AddtoViewport _output_get_2 0)
          (Variables|/Script/Engine.PlayerController|SetbShowMouseCursor Playercontroller true)
          (Input|SetInputModeGameandUI Playercontroller 0 "DoNotLock" true false))))))

(fn AddtoInventory
  (params (Item%20to%20Add :type I%20Tem%20Structure%20Structure) (Quantity :type Integer))
  (bind _inventoryitems (Variables|Default|GetInventoryItems))
  ;[0 1 0.09343] Add to inventory, first we checK if we allready have the same item and that maxstacking is less, else we make new stack
  (bind (_array_element _array_index) (Utilities|Array|ForEachLoopwithBreak (Variables|Default|GetInventoryItems) :!label _label)
    (:LoopBody
      (if (and (== (.ItemClass (Utilities|Struct|BreakITemStructure Item%20to%20Add)) (.itemclass (.Item (Utilities|Struct|BreakSlotStructure _array_element)))) (< (.Quantity (Utilities|Struct|BreakSlotStructure _array_element)) (.maxstackable (.Item (Utilities|Struct|BreakSlotStructure _array_element)))))
        (LocalVariables|SetSlotFound true)
        (LocalVariables|SetIndexFound _array_index)
        (goto _label Break)
        (else
          (LocalVariables|SetSlotFound false))))
    (:Completed
      (if (LocalVariables|GetSlotFound)
        (Utilities|Array|SetArrayElem _inventoryitems (LocalVariables|GetIndexFound) (Utilities|Struct|MakeSlotStructure Item%20to%20Add (+ (.quantity (Utilities|Array|Get(acopy) _inventoryitems (LocalVariables|GetIndexFound))) 1)))
        (LocalVariables|SetIndexFound 0)
        (LocalVariables|SetSlotFound false)
        (CallFunction|RefreshInventory (Game|GetPlayerController 0))
        (return true)
        (else
          (bind _success (CallFunction|CreateNewStack Item%20to%20Add))
          (if _success
            (LocalVariables|SetIndexFound 0)
            (LocalVariables|SetSlotFound false)
            (CallFunction|RefreshInventory (Game|GetPlayerController 0))
            (return true)
            (else
              (return false))))))))

(fn CreateNewStack
  (params (ItemToAdd :type I%20Tem%20Structure%20Structure))
  ;[0.1823 1 0] will make new stack if there is space available, else it will return negative and message will come that inventory is full
  (bind (_array_element _array_index) (Utilities|Array|ForEachLoopwithBreak (Variables|Default|GetInventoryItems) :!label _label)
    (:LoopBody
      (if (== (.Quantity (Utilities|Struct|BreakSlotStructure _array_element)) 0)
        (LocalVariables|SetIndex _array_index)
        (goto _label Break)
        (else
          (LocalVariables|SetIndex -1))))
    (:Completed
      (if (!= (LocalVariables|GetIndex) -1)
        (Utilities|Array|SetArrayElem (Variables|Default|GetInventoryItems) (LocalVariables|GetIndex) (Utilities|Struct|MakeSlotStructure ItemToAdd 1))
        (return true)
        (else
          (return false))))))

(fn RefreshInventory
  (params (Playercontroller :type Player%20Controller%20Object%20Reference))
  ;[0 1 0.3386] Easiest way to refresh it is to remove it and put it back, this happends so fast that it works just fine
  (CallFunction|ToggleInventory Playercontroller)
  (CallFunction|ToggleInventory Playercontroller))

(fn RemovefromInventory
  (params (SlotNumber :type Integer) (Quantity%20to%20remove :type Integer))
  (bind _inventoryitems (Variables|Default|GetInventoryItems))
  (bind _output (Utilities|Array|Get(acopy) _inventoryitems SlotNumber))
  ;[1 0.3524 0] will remove an item from slot given, if the quantity is less than 1 it will set it to default empty slot
  (Utilities|Array|SetArrayElem _inventoryitems SlotNumber (Utilities|Struct|MakeSlotStructure (.item _output) (- (.quantity _output) Quantity%20to%20remove)))
  (if (> (.quantity (Utilities|Array|Get(acopy) (Variables|Default|GetInventoryItems) SlotNumber)) 0)
    _
    (else
      (Utilities|Array|SetArrayElem (Variables|Default|GetInventoryItems) SlotNumber (Utilities|Struct|MakeSlotStructure "(ItemThumb_31_8C22C0354A5504DDB309EC97B1A404BC=None,ItemName_6_E20B2F3247420A63383625B34567D08F=NSLOCTEXT(\"[C978D4AD70820FCA2C0CFF920F400047]\", \"447F584B46B56EB4AA5F09BB787F7092\", \"None\"),Description_8_ADC4FE614AA70F8EB00300841979BA8E=NSLOCTEXT(\"[C978D4AD70820FCA2C0CFF920F400047]\", \"DFFF78CD4D9F753CFDD3069FD2A4C897\", \"None\"),MaxStackable_29_002BE6C54CB05BAA7D2364B65E864F47=0,Type_11_9DEB3B0A4034FF8A7725E38A3A80C979=NewEnumerator0,ItemClass_14_1B4F72BC4A39D24ADA9D6E94D3BF4AA2=\"/Script/CoreUObject.Class'/Script/Engine.Actor'\",ValueGiven_19_CC40DA3B446B420FEF6C78AC0B5419AA=0.000000,LevelNeeded_21_44E9EFC4499E03AD63765B8C046E957D=0,XpGiven_23_3812F9FD4DA6F6E5381D31BE3D23DDE6=0,Mesh_26_762E250D4919D907F1102FBC8718EE7C=None,ClothType_35_0A5DAC2746D25DCF2B478F815AD675F5=NewEnumerator0,ChaosCloth_37_0DD1CC9740B4A7028FB12DAC51D76198=None)"))))
  (CallFunction|RefreshInventory (Game|GetPlayerController 0))
  (return true))

(fn Querry
  (params (item :type Slot%20Structure%20Structure))
  ;[1 0.4852 0.001195] check if we got certain item in our inventory
  (bind (_array_element _array_index) (Utilities|Array|ForEachLoopwithBreak (Variables|Default|GetInventoryItems) :!label _label)
    (:LoopBody
      (if (and (>= (.quantity item) (.quantity _array_element)) (== (.itemclass (.item _array_element)) (.ItemClass (Utilities|Struct|BreakITemStructure (.item item)))))
        (LocalVariables|SetFound (and (>= (.quantity item) (.quantity _array_element)) (== (.itemclass (.item _array_element)) (.ItemClass (Utilities|Struct|BreakITemStructure (.item item))))))
        (LocalVariables|SetSlotnumner _array_index)
        (goto _label Break)))
    (:Completed
      (if (LocalVariables|GetFound)
        (return (LocalVariables|GetFound) (LocalVariables|GetSlotnumner))
        (else
          (return false -1))))))

(fn FindStack
  (params (Item :type I%20Tem%20Structure%20Structure) (quantity :type Integer))
  (bind (_array_element _array_index) (Utilities|Array|ForEachLoopwithBreak (Variables|Default|GetInventoryItems) :!label _label)
    (:LoopBody
      (if (and (== (.itemclass Item) (.itemclass (.item _array_element))) (>= (.quantity _array_element) quantity))
        (LocalVariables|SetLocalFound true)
        (LocalVariables|SetLocalIndex _array_index)
        (LocalVariables|SetLocalAmmount (.quantity _array_element))
        (goto _label Break)))
    (:Completed
      (return (LocalVariables|GetLocalFound) (LocalVariables|GetLocalIndex) (LocalVariables|GetLocalAmmount)))))

(fn RemovebyCrafting
  (params (RemoveArray :type Array%20of%20Remove%20Struct%20Structures) (Playercontroller :type Player%20Controller%20Object%20Reference))
  (for _array_element RemoveArray
    (bind _success (CallFunction|RemovefromInventory (.slotnumber _array_element) (.quantity _array_element)))
    (if _success
      (CallFunction|RefreshInventory Playercontroller))))