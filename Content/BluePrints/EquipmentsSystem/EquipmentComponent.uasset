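; Equipment component that manages armor and clothing on the player's Base_Character, cached from player controller 0 at BeginPlay.
; AddEquipment fills an empty slot, or replaces an occupied one only after the old item goes into the backpack inventory.
; Each change reapplies every fixed-index slot to its body-part static mesh.
; AddClothes overwrites its slot directly and reapplies Chaos Cloth assets to top, bottom and boots.
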(event EventBeginPlay
  (bind _asbase_character (Utilities|Casting|CastToBase_Character (Pawn|GetControlledPawn (Game|GetPlayerController 0))))
  (Variables|Default|SetCharacter _asbase_character))

(fn AddEquipment
  (params (ItemToAdd :type Slot%20Structure%20Structure) (Index :type Integer))
  (bind _equipmentarray (Variables|Default|GetEquipmentArray))
  (bind _character (Variables|Default|GetCharacter))
  (bind _output (Utilities|Array|Get(acopy) _equipmentarray Index))
  (bind _backpackref (Variables|/Game/BluePrints/Characters/Base_Character.Base_Character_C|GetBackPackRef _character))
  (if (== (.quantity _output) 0)
    (Utilities|Array|SetArrayElem _equipmentarray Index ItemToAdd :!label _label)
    (CallFunction|SetArmorMeshes)
    (else
      (Utilities|IsValid _backpackref
        (:Is%20Valid
          (bind _success (Default|AddtoInventory (Variables|/Game/BluePrints/InventorySystem/PlayerInventories/BackPack_Master.BackPack_Master_C|GetInventoryComponent _backpackref) (.item _output) (.quantity _output)))
          (if _success
            (goto _label)))))))

(fn AddClothes
  (params (ClothesToAdd :type Slot%20Structure%20Structure) (Index :type Integer))
  (Utilities|Array|SetArrayElem (Variables|Default|GetClothesArray) Index ClothesToAdd)
  (CallFunction|SetClothesAssets))

(fn SetArmorMeshes
  ;[0 0.09409 1] Function that sets the actual mesh on character
  (Utilities|FlowControl|Sequence
    (:then_0
      ;;[1 0.9451 0] HEAD
      (Components|StaticMesh|SetStaticMesh (Variables|/Game/BluePrints/Characters/Base_Character.Base_Character_C|GetHead (Variables|Default|GetCharacter)) (.mesh (.item (Utilities|Array|Get(acopy) (Variables|Default|GetEquipmentArray))))))
    (:then_1
      ;;[1 0.9693 0.02591] EYES
      (Components|StaticMesh|SetStaticMesh (Variables|/Game/BluePrints/Characters/Base_Character.Base_Character_C|GetEyes (Variables|Default|GetCharacter)) (.mesh (.item (Utilities|Array|Get(acopy) (Variables|Default|GetEquipmentArray) 1)))))
    (:then_2
      ;;[1 0.9906 0] FACE
      (Components|StaticMesh|SetStaticMesh (Variables|/Game/BluePrints/Characters/Base_Character.Base_Character_C|GetFace (Variables|Default|GetCharacter)) (.mesh (.item (Utilities|Array|Get(acopy) (Variables|Default|GetEquipmentArray) 2)))))
    (:then_3
      ;;[1 0.8284 0] NECK
      (Components|StaticMesh|SetStaticMesh (Variables|/Game/BluePrints/Characters/Base_Character.Base_Character_C|GetNeck (Variables|Default|GetCharacter)) (.mesh (.item (Utilities|Array|Get(acopy) (Variables|Default|GetEquipmentArray) 3)))))
    (:then_4
      ;;[0.9779 1 0] LeftShoulder
      (Components|StaticMesh|SetStaticMesh (Variables|/Game/BluePrints/Characters/Base_Character.Base_Character_C|GetLShoulder (Variables|Default|GetCharacter)) (.mesh (.item (Utilities|Array|Get(acopy) (Variables|Default|GetEquipmentArray) 4)))))
    (:then_5
      ;;[1 0.8572 0.03399] RighShoulder
      (Components|StaticMesh|SetStaticMesh (Variables|/Game/BluePrints/Characters/Base_Character.Base_Character_C|GetRShoulder (Variables|Default|GetCharacter)) (.mesh (.item (Utilities|Array|Get(acopy) (Variables|Default|GetEquipmentArray) 5)))))
    (:then_6
      ;;[1 1 1] CHEST
      (Components|StaticMesh|SetStaticMesh (Variables|/Game/BluePrints/Characters/Base_Character.Base_Character_C|GetChest (Variables|Default|GetCharacter)) (.mesh (.item (Utilities|Array|Get(acopy) (Variables|Default|GetEquipmentArray) 6)))))
    (:then_7
      ;;[1 1 1] LeftupperArm
      (Components|StaticMesh|SetStaticMesh (Variables|/Game/BluePrints/Characters/Base_Character.Base_Character_C|GetL_UpperArm (Variables|Default|GetCharacter)) (.mesh (.item (Utilities|Array|Get(acopy) (Variables|Default|GetEquipmentArray) 7)))))
    (:then_8
      ;;[1 1 1] RightupperArm
      (Components|StaticMesh|SetStaticMesh (Variables|/Game/BluePrints/Characters/Base_Character.Base_Character_C|GetR_UpperArm (Variables|Default|GetCharacter)) (.mesh (.item (Utilities|Array|Get(acopy) (Variables|Default|GetEquipmentArray) 8)))))
    (:then_9
      ;;[1 1 1] LeftUpperArm
      (Components|StaticMesh|SetStaticMesh (Variables|/Game/BluePrints/Characters/Base_Character.Base_Character_C|GetR_UpperArm (Variables|Default|GetCharacter)) (.mesh (.item (Utilities|Array|Get(acopy) (Variables|Default|GetEquipmentArray) 9)))))
    (:then_10
      ;;[1 1 1] RightElbow
      (Components|StaticMesh|SetStaticMesh (Variables|/Game/BluePrints/Characters/Base_Character.Base_Character_C|GetRElbow (Variables|Default|GetCharacter)) (.mesh (.item (Utilities|Array|Get(acopy) (Variables|Default|GetEquipmentArray) 10)))))
    (:then_11
      ;;[1 1 1] LeftElbow
      (Components|StaticMesh|SetStaticMesh (Variables|/Game/BluePrints/Characters/Base_Character.Base_Character_C|GetLElbow (Variables|Default|GetCharacter)) (.mesh (.item (Utilities|Array|Get(acopy) (Variables|Default|GetEquipmentArray) 11)))))
    (:then_12
      ;;[1 1 1] LeftElbow
      (Components|StaticMesh|SetStaticMesh (Variables|/Game/BluePrints/Characters/Base_Character.Base_Character_C|GetLElbow (Variables|Default|GetCharacter)) (.mesh (.item (Utilities|Array|Get(acopy) (Variables|Default|GetEquipmentArray) 12)))))
    (:then_13
      ;;[1 1 1] LeftLowerArm
      (Components|StaticMesh|SetStaticMesh (Variables|/Game/BluePrints/Characters/Base_Character.Base_Character_C|GetL_LowerArm (Variables|Default|GetCharacter)) (.mesh (.item (Utilities|Array|Get(acopy) (Variables|Default|GetEquipmentArray) 13)))))
    (:then_14
      ;;[1 1 1] Rightlowerarm
      (Components|StaticMesh|SetStaticMesh (Variables|/Game/BluePrints/Characters/Base_Character.Base_Character_C|GetR_LowerArm (Variables|Default|GetCharacter)) (.mesh (.item (Utilities|Array|Get(acopy) (Variables|Default|GetEquipmentArray) 14)))))
    (:then_15
      ;;[1 1 1] waist
      (Components|StaticMesh|SetStaticMesh (Variables|/Game/BluePrints/Characters/Base_Character.Base_Character_C|GetWaist (Variables|Default|GetCharacter)) (.mesh (.item (Utilities|Array|Get(acopy) (Variables|Default|GetEquipmentArray) 15)))))
    (:then_16
      ;;[1 1 1] Lefthand
      (Components|StaticMesh|SetStaticMesh (Variables|/Game/BluePrints/Characters/Base_Character.Base_Character_C|GetLHand (Variables|Default|GetCharacter)) (.mesh (.item (Utilities|Array|Get(acopy) (Variables|Default|GetEquipmentArray) 16)))))
    (:then_17
      ;;[1 1 1] Righthand
      (Components|StaticMesh|SetStaticMesh (Variables|/Game/BluePrints/Characters/Base_Character.Base_Character_C|GetRHand (Variables|Default|GetCharacter)) (.mesh (.item (Utilities|Array|Get(acopy) (Variables|Default|GetEquipmentArray) 17)))))
    (:then_18
      ;;[1 1 1] LeftUpperLeg
      (Components|StaticMesh|SetStaticMesh (Variables|/Game/BluePrints/Characters/Base_Character.Base_Character_C|GetL_UpperLeg (Variables|Default|GetCharacter)) (.mesh (.item (Utilities|Array|Get(acopy) (Variables|Default|GetEquipmentArray) 18)))))
    (:then_19
      ;;[1 1 1] RightUpperLeg
      (Components|StaticMesh|SetStaticMesh (Variables|/Game/BluePrints/Characters/Base_Character.Base_Character_C|GetR_UpperLeg (Variables|Default|GetCharacter)) (.mesh (.item (Utilities|Array|Get(acopy) (Variables|Default|GetEquipmentArray) 19)))))
    (:then_20
      ;;[1 1 1] LeftKnee
      (Components|StaticMesh|SetStaticMesh (Variables|/Game/BluePrints/Characters/Base_Character.Base_Character_C|GetL_knee (Variables|Default|GetCharacter)) (.mesh (.item (Utilities|Array|Get(acopy) (Variables|Default|GetEquipmentArray) 20)))))
    (:then_21
      ;;[1 1 1] RightKnee
      (Components|StaticMesh|SetStaticMesh (Variables|/Game/BluePrints/Characters/Base_Character.Base_Character_C|GetR_Knee (Variables|Default|GetCharacter)) (.mesh (.item (Utilities|Array|Get(acopy) (Variables|Default|GetEquipmentArray) 21)))))
    (:then_22
      ;;[1 1 1] LeftLowerLeg
      (Components|StaticMesh|SetStaticMesh (Variables|/Game/BluePrints/Characters/Base_Character.Base_Character_C|GetL_lowLeg (Variables|Default|GetCharacter)) (.mesh (.item (Utilities|Array|Get(acopy) (Variables|Default|GetEquipmentArray) 22)))))
    (:then_23
      ;;[1 1 1] RightLowerLeg
      (Components|StaticMesh|SetStaticMesh (Variables|/Game/BluePrints/Characters/Base_Character.Base_Character_C|GetR_LowLeg (Variables|Default|GetCharacter)) (.mesh (.item (Utilities|Array|Get(acopy) (Variables|Default|GetEquipmentArray) 23)))))
    (:then_24
      ;;[1 1 1] LeftToe
      (Components|StaticMesh|SetStaticMesh (Variables|/Game/BluePrints/Characters/Base_Character.Base_Character_C|GetL_Toe (Variables|Default|GetCharacter)) (.mesh (.item (Utilities|Array|Get(acopy) (Variables|Default|GetEquipmentArray) 24)))))
    (:then_25
      ;;[1 1 1] RightToe
      (Components|StaticMesh|SetStaticMesh (Variables|/Game/BluePrints/Characters/Base_Character.Base_Character_C|GetRtoe (Variables|Default|GetCharacter)) (.mesh (.item (Utilities|Array|Get(acopy) (Variables|Default|GetEquipmentArray) 25)))))))

(fn SetClothesAssets
  (Utilities|FlowControl|Sequence
    (:then_0
      (Class|ChaosClothComponent|SetClothAsset (Variables|/Game/BluePrints/Characters/Base_Character.Base_Character_C|GetTop (Variables|Default|GetCharacter)) (.chaoscloth (.item (Utilities|Array|Get(acopy) (Variables|Default|GetClothesArray))))))
    (:then_1
      (Class|ChaosClothComponent|SetClothAsset (Variables|/Game/BluePrints/Characters/Base_Character.Base_Character_C|GetBottom (Variables|Default|GetCharacter)) (.chaoscloth (.item (Utilities|Array|Get(acopy) (Variables|Default|GetClothesArray) 1)))))
    (:then_2
      (Class|ChaosClothComponent|SetClothAsset (Variables|/Game/BluePrints/Characters/Base_Character.Base_Character_C|GetBoots (Variables|Default|GetCharacter)) (.chaoscloth (.item (Utilities|Array|Get(acopy) (Variables|Default|GetClothesArray) 2)))))))